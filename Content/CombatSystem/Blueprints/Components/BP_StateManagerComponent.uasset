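; State manager component for the combat system that tracks its owner's current state and current character action.
; SetState and SetCurrentAction ignore unchanged values, otherwise firing an End event for the old value and a Begin event for the new one.
; Getters and Contains-based checks let other logic query either value, and ResetState returns only the state to a fixed enum entry.
; It is purely call-driven, with no active BeginPlay or Tick logic.
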(event EventBeginPlay)

(event EventTick
  (params (DeltaSeconds :type Float%20%28single-precision%29)))

(fn SetState
  (params (NewState :type E_CharacterStates%20Enum :default "NewEnumerator0"))
  (if (Utilities|Enum|NotEqual(Enum) NewState (Variables|Default|GetCurrentState))
    (Default|CallOnStateEnd (Variables|Default|GetCurrentState))
    (bind _output_get (Variables|Default|SetCurrentState NewState))
    (Default|CallOnStateBegin _output_get)))

(fn GetCurrentState
  (return (Variables|Default|GetCurrentState)))

(fn ResetState
  (CallFunction|SetState "NewEnumerator0"))

(fn IsCurrentStateEqualtoAny?
  (params (StatesToCheck :type Array%20of%20E_CharacterStates%20Enums :default "NewEnumerator0"))
  (return (Utilities|Array|ContainsItem StatesToCheck (Variables|Default|GetCurrentState))))

(fn SetCurrentAction
  (params (NewCharacterAction :type E_CharacterActions%20Enum :default "NewEnumerator0"))
  (if (Utilities|Enum|NotEqual(Enum) NewCharacterAction (Variables|Default|GetCurrentCharacterAction))
    (Default|CallOnCharacterActionEnd (Variables|Default|GetCurrentCharacterAction))
    (bind _output_get (Variables|Default|SetCurrentCharacterAction NewCharacterAction))
    (Default|CallOnCharacterActionBegin _output_get)))

(fn GetCurrentAction
  (return (Variables|Default|GetCurrentCharacterAction)))

(fn IsCurrentActionEqualtoAny?
  (params (ActionsToCheck :type Array%20of%20E_CharacterActions%20Enums :default "NewEnumerator0"))
  (return (Utilities|Array|ContainsItem ActionsToCheck (Variables|Default|GetCurrentCharacterAction))))