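; Combat hit-detection component that sweeps a sphere trace between two sockets on an assigned mesh while collisions are active.
; Tick runs the multi-sphere object trace, skipping listed ignored actors, and fires OnHit for each valid hit.
; Each actor registers only once per activation, as activating clears the already-hit list.
; An optional gameplay tag filter excludes actors owning any of the ignored tags.
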(event Custom|ActivateCollisions
  ;[1 1 1] Activate Collisions
  (CallFunction|ClearHitActors)
  (Variables|Default|SetbIsCollisionEnabled? true))

(event Custom|DeactivateCollisions
  ;[1 1 1] Deactivate Collisions
  (Variables|Default|SetbIsCollisionEnabled? false))

(event Custom|CollisionsTrace
  ;[1 1 1] Collisions Trace
  (bind _outhits (Collision|MultiSphereTraceForObjects (Transformation|GetSocketLocation (Variables|Default|GetCollisionMeshComponent) (Variables|Initialization|GetStartSocketName)) (Transformation|GetSocketLocation (Variables|Default|GetCollisionMeshComponent) (Variables|Initialization|GetEndSocketName)) (Variables|Initialization|GetTraceRadius) (Variables|Initialization|GetCollisionObjectTypes) false (Variables|Default|GetActors%20to%20Ignore) (Variables|Initialization|GetDraw%20Debug%20Type)))
  (for _array_element _outhits
    (bind _output_get (Variables|Default|SetLastHit _array_element))
    (if (CallFunction|CanHitActor? (.HitActor (Collision|BreakHitResult _output_get)))
      (bind _output_get_2 (Variables|Default|SetHit%20Actor (.HitActor (Collision|BreakHitResult _output_get))))
      (Utilities|Array|Add (Variables|Default|GetAlreadyHitActors) _output_get_2)
      (Default|CallOnHit (Variables|Default|GetLastHit)))))

(event Custom|ClearHitActors
  ;[1 1 1] Clear Hit Actors
  (Utilities|Array|Clear (Variables|Default|GetAlreadyHitActors)))

(event Custom|SetCollisionMesh
  (params (MeshComponent :type Primitive%20Component%20Object%20Reference))
  ;[1 1 1] Set Collision Mesh
  (Variables|Default|SetCollisionMeshComponent MeshComponent))

(event EventBeginPlay)

(event EventTick
  (params (DeltaSeconds :type Float%20%28single-precision%29))
  (if (Variables|Default|GetbIsCollisionEnabled?)
    (CallFunction|CollisionsTrace)))

(fn GetAlreadyHitActors
  (return (Variables|Default|GetAlreadyHitActors)))

(fn IsCollisionEnabled
  (return (Variables|Default|GetbIsCollisionEnabled?)))

(fn GetLastHit
  (return (Variables|Default|GetLastHit)))

(fn GetCollisionMeshComponent
  (return (Variables|Default|GetCollisionMeshComponent)))

(fn AddActortoIgnore
  (params (ActorToIgnore :type Actor%20Object%20Reference%20%28by%20ref%29))
  (Utilities|Array|AddUnique (Variables|Default|GetActors%20to%20Ignore) ActorToIgnore))

(fn RemoveActortoIgnore
  (params (ActorToRemove :type Actor%20Object%20Reference%20%28by%20ref%29))
  (Utilities|Array|RemoveItem (Variables|Default|GetActors%20to%20Ignore) ActorToRemove))

(fn GetActorstoIgnore
  (return (Variables|Default|GetActors%20to%20Ignore)))

(fn CanHitActor?
  (params (InActor :type Actor%20Object%20Reference%20%28by%20ref%29))
  (if (Variables|Initialization|GetbShouldIgnoreOtherActors)
    (bind _returnvalue (Class|BPIGameplayTag|GetOwnedGameplayTags(Message) InActor))
    (return (and (not (GameplayTags|HasAnyTags _returnvalue (Variables|Default|GetGameplayTagsToIgnore) true)) (not (Utilities|Array|ContainsItem (Variables|Default|GetAlreadyHitActors) InActor))))
    (else
      (return (not (Utilities|Array|ContainsItem (Variables|Default|GetAlreadyHitActors) InActor))))))