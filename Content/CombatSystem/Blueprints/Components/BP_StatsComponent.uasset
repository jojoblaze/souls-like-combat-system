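; Actor component that holds a character's stats, such as Health and Stamina, for the combat system.
; Base/max and current values live in maps keyed by stat, with current-value writes broadcasting an update event.
; Clamped modifications can start stamina regeneration, a looping timer behind a retriggerable delay that stops at max.
; TakeDamage reduces Health and, at zero, changes the owner's state through BP_StateManagerComponent.
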(event Custom|StartRegen
  (params (Stat :type E_Stats%20Enum :default "NewEnumerator0"))
  (switch Utilities|FlowControl|Switch|SwitchonE_Stats Stat
    (:NewEnumerator2
      (Utilities|Time|ClearTimerbyFunctionName 0 "RegenStamina")
      (Utilities|FlowControl|RetriggerableDelay 1.5)
      (Utilities|Time|SetTimerbyFunctionName 0 "RegenStamina" 0.1 true))))

(event EventBeginPlay)

(event EventTick
  (params (DeltaSeconds :type Float%20%28single-precision%29)))

(fn SetCurrentStatValue
  (params (Stat :type E_Stats%20Enum :default "NewEnumerator0") (Value :type Float%20%28double-precision%29))
  (Utilities|Map|Add (Variables|Default|GetCurrentStats) Stat Value)
  (Default|CallOnCurrentStatValueUpdated Stat Value))

(fn GetCurrentStatValue
  (params (Stat :type E_Stats%20Enum :default "NewEnumerator0"))
  (return (.Value (Utilities|Map|Find (Variables|Default|GetCurrentStats) Stat))))

(fn InitializeStats
  (bind _keys (Utilities|Map|Keys (Variables|BaseStats|GetBaseStats)))
  (for _array_element _keys
    (CallFunction|SetCurrentStatValue _array_element (.basevalue (.Value (Utilities|Map|Find (Variables|BaseStats|GetBaseStats) _array_element))))))

(fn ModifyCurrentStatValue
  (params (Stat :type E_Stats%20Enum :default "NewEnumerator0") (Value :type Float%20%28double-precision%29) (bShouldRegenerate :type Boolean))
  (if (!= Value 0.0)
    (bind _output_get (LocalVariables|SetL_Value (Math|Float|Clamp(Float) (+ (CallFunction|GetCurrentStatValue Stat) Value) 0.0 (BaseStats|GetMaxStatValue Stat))))
    (CallFunction|SetCurrentStatValue Stat _output_get)
    (if bShouldRegenerate
      (CallFunction|StartRegen Stat))))

(fn SetBaseStatValue
  (params (Stat :type E_Stats%20Enum :default "NewEnumerator0") (Value :type Float%20%28double-precision%29))
  (bind _structout (Utilities|Struct|SetmembersinF_BaseStat (.Value (Utilities|Map|Find (Variables|BaseStats|GetBaseStats) Stat)) Value))
  (Utilities|Map|Add (Variables|BaseStats|GetBaseStats) Stat _structout))

(fn GetBaseStatValue
  (params (Stat :type E_Stats%20Enum :default "NewEnumerator0"))
  (return (.basevalue (.Value (Utilities|Map|Find (Variables|BaseStats|GetBaseStats) Stat)))))

(fn GetMaxStatValue
  (params (Stat :type E_Stats%20Enum :default "NewEnumerator0"))
  (return (.maxvalue (.Value (Utilities|Map|Find (Variables|BaseStats|GetBaseStats) Stat)))))

(fn SetMaxStatValue
  (params (Stat :type E_Stats%20Enum :default "NewEnumerator0") (Value :type Float%20%28double-precision%29))
  (bind _structout (Utilities|Struct|SetmembersinF_BaseStat (.Value (Utilities|Map|Find (Variables|BaseStats|GetBaseStats) Stat)) Value))
  (Utilities|Map|Add (Variables|BaseStats|GetBaseStats) Stat _structout))

(fn TakeDamage
  (params (InDamage :type Float%20%28double-precision%29))
  (Development|PrintText (Utilities|Text|FormatText "current health: {health}" (CallFunction|GetCurrentStatValue "NewEnumerator1")) true true "(R=0.570312,G=0.483644,B=0.006653,A=1.000000)" 1e+01)
  (CallFunction|ModifyCurrentStatValue "NewEnumerator1" (* InDamage -1.0) false)
  (if (<= (CallFunction|GetCurrentStatValue "NewEnumerator1") 0.0)
    (Default|SetState (Actor|GetComponentbyClass (Components|GetOwner) "/Game/CombatSystem/Blueprints/Components/BP_StateManagerComponent.BP_StateManagerComponent_C") "NewEnumerator4")))

(fn RegenStamina
  (CallFunction|SetCurrentStatValue "NewEnumerator2" (Math|Float|Clamp(Float) (+ (CallFunction|GetCurrentStatValue "NewEnumerator2") (Variables|StatsRegen|GetStaminaRegenRate)) 0.0 (BaseStats|GetMaxStatValue "NewEnumerator2")))
  (if (>= (CallFunction|GetCurrentStatValue "NewEnumerator2") (BaseStats|GetMaxStatValue "NewEnumerator2"))
    (Utilities|Time|ClearTimerbyFunctionName 0 "RegenStamina")))